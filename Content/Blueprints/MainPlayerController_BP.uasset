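; Player controller Blueprint that adds fade transitions to the pause menu display and removal events inherited from its parent class.
; On display, it runs the parent logic, casts the menu widget to PauseMenu, stores the reference and plays its FadeIn animation.
; On removal, it runs the parent logic, plays FadeIn in reverse and hides the widget after a short delay.
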(event EventBeginPlay)

(event EventTick
  (params (DeltaSeconds :type Float%20%28single-precision%29)))

(event EventDisplayPauseMenu
  (|CallParentFunction)
  (bind _aspause_menu (Utilities|Casting|CastToPauseMenu (Variables|Default|GetPauseMenu)))
  (bind _output_get (Variables|Default|SetRefToPauseMenu _aspause_menu))
  (UserInterface|Animation|PlayAnimation _output_get (Variables|/Game/Blueprints/HUD/PauseMenu.PauseMenu_C|GetFadeIn _aspause_menu) 0.0 1 "Forward" 1.0 false)
  (Utilities|FlowControl|Delay 0.25))

(event EventRemovePauseMenu
  (bind _reftopausemenu (Variables|Default|GetRefToPauseMenu))
  (|CallParentFunction)
  (UserInterface|Animation|PlayAnimation _reftopausemenu (Variables|/Game/Blueprints/HUD/PauseMenu.PauseMenu_C|GetFadeIn _reftopausemenu) 0.0 1 "Reverse" 1.0 false)
  (Utilities|FlowControl|Delay 0.25)
  (Widget|SetVisibility (Variables|Default|GetRefToPauseMenu) "Hidden"))

(event Input|KeyboardEvents|Q
  (params (Key :type Key%20Structure :default "None")))

(event Input|KeyboardEvents|Escape
  (params (Key :type Key%20Structure :default "None")))

(fn ConstructionScript)